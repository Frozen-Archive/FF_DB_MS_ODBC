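; Template actor that demonstrates the MS ODBC SQL plugin by running a test query against a SQL database at BeginPlay.
; It spawns an MS_ODBC_Manager, connects using server and credentials from the GI_Plugins game instance, then sends a fixed SELECT.
; F_Query_View prints each result row via F_Recurse_Row, with success-colored status messages.
; Disconnected snippets sample other result APIs such as metadata, column and single-cell reads, some using F_Writer.
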(event EventBeginPlay
  (bind _returnvalue (Game|SpawnActorfromClass "/Script/FF_DB_MS_ODBC.MS_ODBC_Manager" (Math|Transform|MakeTransform "0, 0, 0" "0, 0, 0" "1.000000,1.000000,1.000000") "Undefined" "MultiplyWithRoot" 0 0))
  (Variables|Default|SetSQL_Manager _returnvalue)
  (bind _asgi_plugins (Utilities|Casting|CastToGI_Plugins (Game|GetGameInstance)))
  (bind (_out_connection _out_code _createdstring _returnvalue_2) (Class|MSODBCManager|CreateConnection (Variables|Default|GetSQL_Manager) (.Value (Utilities|Map|Find (Variables|/Game/Player/GI_Plugins.GI_Plugins_C|GetODBC_Servers _asgi_plugins) "home")) (.Value (Utilities|Map|Find (Variables|/Game/Player/GI_Plugins.GI_Plugins_C|GetUsers _asgi_plugins) "odbc")) (.Value (Utilities|Map|Find (Variables|/Game/Player/GI_Plugins.GI_Plugins_C|GetPasswords _asgi_plugins) "odbc"))))
  (Development|PrintString _out_code true true (Math|Color|SelectColor "(R=0.000000,G=1.000000,B=0.000000,A=1.000000)" "(R=1.000000,G=0.000000,B=0.000000,A=1.000000)" _returnvalue_2) 6e+01)
  (bind (_out_code_2 _out_result _returnvalue_3) (Class|MSODBCConnection|SendQuery _out_connection "SELECT stamp FROM ue5_test.dbo.Table_1" true))
  (Development|PrintString _out_code_2 true true (Math|Color|SelectColor "(R=0.000000,G=1.000000,B=0.000000,A=1.000000)" "(R=1.000000,G=0.000000,B=0.000000,A=1.000000)" _returnvalue_3) 6e+01)
  (Queries|FQueryView _out_result))

(fn ConstructionScript)

(fn FQueryView
  (params (In_Result :type MS%20ODBC%20Result%20Object%20Reference))
  (bind _output_get (LocalVariables|SetLOC_Result In_Result))
  (Utilities|IsValid _output_get
    (:Is%20Valid
      (for _index (range 0 (- (Class|MSODBCResult|GetRowNumber (LocalVariables|GetLOC_Result)) 1))
        (bind (_out_code _out_values _returnvalue) (Class|MSODBCResult|GetRow (LocalVariables|GetLOC_Result) _index))
        (Development|PrintString _out_code true true (Math|Color|SelectColor "(R=0.000000,G=1.000000,B=0.000000,A=1.000000)" "(R=1.000000,G=0.000000,B=0.000000,A=1.000000)" _returnvalue) 6e+01)
        (if _returnvalue
          (bind _returnvalue_2 (Helpers|FRecurseRow _out_values " // "))
          (Development|PrintString _returnvalue_2 true true "(R=0.000000,G=0.660000,B=1.000000,A=1.000000)" 6e+01)))
      (return))
    (:Is%20Not%20Valid
      (return))))

(fn FRecurseRow
  (params (In_Array :type Array%20of%20MS%20ODBC%20Data%20Value%20Structures) (Seperator :type String))
  (for _array_element In_Array
    (Utilities|Array|Add (LocalVariables|GetEach_Row) (Utilities|String|Append (Utilities|String|ToString(Integer) (.datatype _array_element)) " = " (.columnname _array_element) " = " (.preview _array_element))))
  (return (Utilities|String|JoinStringArray (LocalVariables|GetEach_Row) Seperator)))

(fn FWriter
  (params (In_Code :type String) (Array :type Array%20of%20MS%20ODBC%20Data%20Value%20Structures) (bIsSuccessfull :type Boolean))
  (Development|PrintString In_Code true true (Math|Color|SelectColor "(R=0.000000,G=1.000000,B=0.000000,A=1.000000)" "(R=1.000000,G=0.000000,B=0.000000,A=1.000000)" bIsSuccessfull) 6e+01)
  (if bIsSuccessfull
    (for _array_element Array
      (Development|PrintString (.preview _array_element) true true "(R=0.000000,G=0.660000,B=1.000000,A=1.000000)" 6e+01))
    (return)
    (else
      (return))))